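; BP_GameModeBase is a game mode that opens the main menu and owns the background music.
; On BeginPlay it switches to windowed mode, creates the 2D music sound without playing it, and shows WBP_MainMenu with UI-only input and a visible cursor.
; Playmusic and Stopmusic events start and stop the stored music component, with no caller in this graph.
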(event `self.ReceiveBeginPlay`
  (bind _returnvalue (`GameplayStatics.GetPlayerController` 0))
  (bind _returnvalue_2 (`GameUserSettings.GetGameUserSettings`))
  (`GameUserSettings.SetFullscreenMode` _returnvalue_2 "Windowed")
  (`GameUserSettings.ApplyResolutionSettings` _returnvalue_2 false)
  (bind _returnvalue_3 (`GameplayStatics.CreateSound2D` "/Game/Assets/Music/Japanese_Fantasy_Music_-_Bushido.Japanese_Fantasy_Music_-_Bushido" 1.0 1.0 0.0 null))
  (set `self.Music` _returnvalue_3)
  (bind _returnvalue_4 (`|CreateWidget` "/Game/Blueprints/Widgets/WBP_MainMenu.WBP_MainMenu_C"))
  (`UserWidget.AddToViewport` _returnvalue_4 0)
  (`WidgetBlueprintLibrary.SetInputMode_UIOnlyEx` _returnvalue _returnvalue_4)
  (set `PlayerController.bShowMouseCursor` true _returnvalue))

(event `Play music`
  (`AudioComponent.Play` (`self.Music`) 0.0))

(event `Stop music`
  (`AudioComponent.Stop` (`self.Music`)))

(fn `UserConstructionScript`)