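; BP_VillageDoor is a door actor that moves along a referenced spline when its UnlockVillage event fires.
; UnlockVillage calls MoveObject, which scales a timeline's play rate to a configurable duration in seconds and plays it from the start.
; Each update maps the timeline track to a distance along the spline, moving the actor there while keeping the mesh's world rotation and scale.
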(event `UnlockVillage`
  (`self.Move Object`))

(event `Move Object`
  (bind _staticmeshcomponent0 (`self.StaticMeshComponent0`))
  ;[1 1 1] Move Object (following a spline)
  (`TimelineComponent.SetPlayRate` (`self.Move Object T`) (/ 1.0 (`self.Time To Complete (in seconds)`)))
  (bind (_direction _move_track) (`Timeline|Move Object T` :!via `PlayFromStart`)
    (:`Update`
      (`self.K2_SetActorTransform` (`KismetMathLibrary.MakeTransform` (`SplineComponent.GetLocationAtDistanceAlongSpline` (`/Game/Blueprints/History_CP_BP/Spline/BP_SplinePath.Spline` (`self.SplineRef`)) (`KismetMathLibrary.Lerp` 0.0 (`SplineComponent.GetSplineLength` (`/Game/Blueprints/History_CP_BP/Spline/BP_SplinePath.Spline` (`self.SplineRef`))) _move_track) "World") (`SceneComponent.K2_GetComponentRotation` _staticmeshcomponent0) (`SceneComponent.K2_GetComponentScale` _staticmeshcomponent0))))))

(fn `UserConstructionScript`)