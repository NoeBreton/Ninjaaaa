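; BP_TriggerBox is a trigger volume that fires one enum-selected event when the player or a BlackKnightBlade projectile overlaps its box.
; On overlap it hides CPParticule, then switches on TriggerEnum to unlock the village door, kill the player, or move the respawn transform to its Arrow.
; The village door case briefly shows a WBP_History text widget before unlocking.
; The door and respawn triggers destroy themselves after use.
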(event `self.Box.OnComponentBeginOverlap`
  (params (OverlappedComponent :type "PrimitiveComponent Object Reference") (OtherActor :type "Actor Object Reference") (OtherComp :type "PrimitiveComponent Object Reference") (OtherBodyIndex :type Integer) (bFromSweep :type Boolean) (SweepResult :type "HitResult Structure (by ref)"))
  (bind _asbp_player (cast `/Game/Blueprints/CharacterBlueprints/BP_Player` OtherActor)
    (:`then`
      _)
    (:`CastFailed`
      (cast `/Game/Blueprints/WeaponBlueprints/BlackBladeWeapon/BP_BlackKnightBlade_Projectile` OtherActor)))
  (`self.SetActorHiddenInGame` (`self.CPParticule`) true)
  (switch `/Game/Blueprints/Enums/E_TriggerBox` (`self.TriggerEnum`)
    (:`NewEnumerator0`
      (bind _returnvalue (`|CreateWidget` "/Game/Blueprints/HistoryWidgets/WBP_History.WBP_History_C"))
      (set `/Game/Blueprints/HistoryWidgets/WBP_History.Interaction Text` (`self.Interaction Text`) _returnvalue)
      (`UserWidget.AddToViewport` _returnvalue 0)
      (`KismetSystemLibrary.Delay` 3.0)
      (`Widget.RemoveFromParent` _returnvalue)
      (`KismetSystemLibrary.Delay` 1.0)
      (`/Game/Blueprints/History_CP_BP/BP_VillageDoor.UnlockVillage` (`self.VillageDoor`))
      (`self.K2_DestroyActor`))
    (:`NewEnumerator3`
      (`/Game/Blueprints/CharacterBlueprints/BP_Player.Death` _asbp_player))
    (:`NewEnumerator4`
      (`/Game/Blueprints/CharacterBlueprints/BP_Player.ChangeRespawnTransform` _asbp_player (`SceneComponent.K2_GetComponentToWorld` (`self.Arrow`)))
      (`self.K2_DestroyActor`))))

(fn `UserConstructionScript`)