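; Moving platform actor that travels along the spline of a referenced spline actor.
; On BeginPlay it starts a timeline whose play rate is the inverse of TimeToComplete, so that variable controls the travel time.
; Each update maps the timeline's MoveTrack value to a distance along the spline and moves the actor to that world location, keeping the mesh's current rotation and scale.
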(event `self.ReceiveBeginPlay`
  (bind _staticmeshcomponent0 (`self.StaticMeshComponent0`))
  ;[1 1 1] Move Object (following a spline)
  (`TimelineComponent.SetPlayRate` (`self.Timeline`) (/ 1.0 (`self.Time To Complete`)))
  (bind (_direction _move_track) (`Timeline|Timeline` :!via `PlayFromStart`)
    (:`Update`
      (`self.K2_SetActorTransform` (`KismetMathLibrary.MakeTransform` (`SplineComponent.GetLocationAtDistanceAlongSpline` (`/Game/Blueprints/History_CP_BP/Spline/BP_SplinePath.Spline` (`self.Spline Ref`)) (`KismetMathLibrary.Lerp` 0.0 (`SplineComponent.GetSplineLength` (`/Game/Blueprints/History_CP_BP/Spline/BP_SplinePath.Spline` (`self.Spline Ref`))) _move_track) "World") (`SceneComponent.K2_GetComponentRotation` _staticmeshcomponent0) (`SceneComponent.K2_GetComponentScale` _staticmeshcomponent0))))))

(fn `UserConstructionScript`)