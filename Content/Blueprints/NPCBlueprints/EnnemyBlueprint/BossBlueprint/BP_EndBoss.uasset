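; End boss Blueprint that lobs fireballs at the player while they are within its Detection volume.
; A looping 1.5-second timer drives AutoAttack, which turns the boss toward the player and spawns BP_FireBall.
; ArcPrediction leads the moving target by distance-scaled velocity and computes an arced launch velocity.
; Black Knight blade hits call DestroyActor, first showing a timed "climb the tower" message if the boss is invincible.
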(event `Auto Attack`
  ;[1 1 1] Attack when player is detected
  (`KismetSystemLibrary.K2_SetTimerDelegate` (delegate `Auto Attack`) 1.5 true)
  (if (`self.Player Is In Range ?`)
    (`self.Rotate to face player`)
    (bind _desired_velocity (`self.Arc Prediction` (`self.BP Player`)))
    (set `self.Desired Velocity` _desired_velocity)
    (bind _returnvalue (`|SpawnActorFromClass` "/Game/Blueprints/TrapBlueprints/Fireball/BP_FireBall.BP_FireBall_C" (`KismetMathLibrary.MakeTransform` (`SceneComponent.K2_GetComponentLocation` (`self.Projectile Spawn Location`))) "Undefined" "MultiplyWithRoot" null null))
    (`/Engine/EditorBlueprintResources/StandardMacros.IsValid` _returnvalue
      (:`Is Valid`
        (`ProjectileMovementComponent.SetVelocityInLocalSpace` (`/Game/Blueprints/TrapBlueprints/Fireball/BP_FireBall.ProjectileMovement` _returnvalue) (`self.Desired Velocity`))))))

(event `Rotate to face player`
  ;[1 1 1] rotate to face player
  (`self.K2_SetActorRotation` (`KismetMathLibrary.FindRelativeLookAtRotation` (`KismetMathLibrary.Conv_VectorToTransform` (`self.K2_GetActorLocation`)) (`self.K2_GetActorLocation` (`self.BP Player`)))))

(event `self.Detection.OnComponentBeginOverlap`
  (params (OverlappedComponent :type "PrimitiveComponent Object Reference") (OtherActor :type "Actor Object Reference") (OtherComp :type "PrimitiveComponent Object Reference") (OtherBodyIndex :type Integer) (bFromSweep :type Boolean) (SweepResult :type "HitResult Structure (by ref)"))
  ;[1 1 1] Player Detection
  (bind _asbp_player (cast `/Game/Blueprints/CharacterBlueprints/BP_Player` OtherActor))
  (set `self.Player Is In Range ?` true)
  (set `self.BP Player` _asbp_player))

(event `self.Detection.OnComponentEndOverlap`
  (params (OverlappedComponent :type "PrimitiveComponent Object Reference") (OtherActor :type "Actor Object Reference") (OtherComp :type "PrimitiveComponent Object Reference") (OtherBodyIndex :type Integer))
  ;[1 1 1] Player Detection
  (cast `/Game/Blueprints/CharacterBlueprints/BP_Player` OtherActor)
  (set `self.Player Is In Range ?` false))

(event `self.ReceiveBeginPlay`
  (`self.Auto Attack`))

(event `self.BossSensei.OnComponentHit`
  (params (HitComponent :type "PrimitiveComponent Object Reference") (OtherActor :type "Actor Object Reference") (OtherComp :type "PrimitiveComponent Object Reference") (NormalImpulse :type "Vector Structure") (Hit :type "HitResult Structure (by ref)"))
  (cast `/Game/Blueprints/WeaponBlueprints/BlackBladeWeapon/BP_BlackKnightBlade_Projectile` OtherActor)
  (if (`self.Is Invicible ?`)
    (bind _returnvalue (`|CreateWidget` "/Game/Blueprints/HistoryWidgets/WBP_History.WBP_History_C"))
    (set `/Game/Blueprints/HistoryWidgets/WBP_History.Interaction Text` "You need to climb the tower first before doing damage to the boss" _returnvalue)
    (`UserWidget.AddToViewport` _returnvalue 0)
    (`KismetSystemLibrary.Delay` 3.0)
    (`Widget.RemoveFromParent` _returnvalue)
    (`self.K2_DestroyActor`)
    (else
      (`self.K2_DestroyActor`))))

(fn `Arc Prediction`
  (params (Target :type "Actor Object Reference"))
  (returns (`Desired Velocity` :type "Vector Structure"))
  (locals (`Target actor location` :type "Vector Structure") (`Target actor Velocity` :type "Vector Structure"))
  (set `local.Target actor Velocity` (`self.GetVelocity` Target))
  (set `local.Target actor location` (`self.K2_GetActorLocation` Target))
  (bind (_outlaunchvelocity _returnvalue) (`GameplayStatics.SuggestProjectileVelocity_CustomArc` (`SceneComponent.K2_GetComponentLocation` (`self.Projectile Spawn Location`)) (+ (`local.Target actor location`) (* (`local.Target actor Velocity`) (/ (`KismetMathLibrary.Vector_Distance` (`local.Target actor location`) (`self.K2_GetActorLocation`)) 1200.0))) 0.0 0.7))
  (if _returnvalue
    (return _outlaunchvelocity)))

(fn `UserConstructionScript`)