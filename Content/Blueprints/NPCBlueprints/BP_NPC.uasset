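; BP_NPC is an NPC that shows multi-line dialogue when the player is nearby.
; Overlapping InteractBox reveals the key prompt and creates a WBP_DialogueUI widget; leaving hides the prompt and removes it.
; EventDialogueOccurs passes NPCText to the widget, reveals its image and text, then advances the row or closes the widget after the last line.
; A DoOnce guards each step and is reset immediately afterwards.
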(event `self.InteractBox.OnComponentBeginOverlap`
  (params (OverlappedComponent :type "PrimitiveComponent Object Reference") (OtherActor :type "Actor Object Reference") (OtherComp :type "PrimitiveComponent Object Reference") (OtherBodyIndex :type Integer) (bFromSweep :type Boolean) (SweepResult :type "HitResult Structure (by ref)"))
  ;[1 1 1] Open Dialogue When Player Interact
  (cast `/Game/Blueprints/CharacterBlueprints/BP_Player` OtherActor)
  (`SceneComponent.SetHiddenInGame` (`self.InteractKeyText`) false false)
  (bind _returnvalue (`|CreateWidget` "/Game/Blueprints/HistoryWidgets/WBP_DialogueUI.WBP_DialogueUI_C"))
  (bind _output_get (set `self.DialogueUI` _returnvalue))
  (`UserWidget.AddToViewport` _output_get 0))

(event `self.InteractBox.OnComponentEndOverlap`
  (params (OverlappedComponent :type "PrimitiveComponent Object Reference") (OtherActor :type "Actor Object Reference") (OtherComp :type "PrimitiveComponent Object Reference") (OtherBodyIndex :type Integer))
  (bind _dialogueui (`self.DialogueUI`))
  ;[1 1 1] Open Dialogue When Player Interact
  (cast `/Game/Blueprints/CharacterBlueprints/BP_Player` OtherActor)
  (`SceneComponent.SetHiddenInGame` (`self.InteractKeyText`) true false)
  (`/Engine/EditorBlueprintResources/StandardMacros.IsValid` _dialogueui
    (:`Is Valid`
      (`Widget.RemoveFromParent` _dialogueui))))

(event `/Game/Blueprints/Interface/DialogueInterface.EventDialogueOccurs`
  (bind _returnvalue (+ (`/Game/Blueprints/HistoryWidgets/WBP_DialogueUI.DialogueTextRow` (`self.DialogueUI`)) 1))
  ;[1 1 1] Open Dialogue When Player Interact
  (`/Engine/EditorBlueprintResources/StandardMacros.DoOnce` false :!label _label
    (:`Completed`
      (set `/Game/Blueprints/HistoryWidgets/WBP_DialogueUI.DialogueText` (`self.NPCText`) (`self.DialogueUI`))
      (`Widget.SetVisibility` (`/Game/Blueprints/HistoryWidgets/WBP_DialogueUI.Image_40` (`self.DialogueUI`)) "Visible")
      (`Widget.SetVisibility` (`/Game/Blueprints/HistoryWidgets/WBP_DialogueUI.TextBlock_113` (`self.DialogueUI`)) "Visible")
      (if (> _returnvalue (- (`KismetArrayLibrary.Array_Length` (`self.NPCText`)) 1))
        (`Widget.RemoveFromParent` (`self.DialogueUI`))
        (`self.Reset Dialogue`)
        (else
          (set `/Game/Blueprints/HistoryWidgets/WBP_DialogueUI.DialogueTextRow` _returnvalue (`self.DialogueUI`))
          (`self.Reset Dialogue`))))))

(event `Reset Dialogue`
  ;[1 1 1] Open Dialogue When Player Interact
  (goto _label :!via `Reset`))

(fn `UserConstructionScript`)