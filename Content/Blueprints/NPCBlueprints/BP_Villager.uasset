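; BP_Villager is a villager NPC that shows its interaction text when the player presses E nearby.
; A box overlap with BP_Player enables input, creates a WBP_History widget carrying the villager's InteractionText, and opens a gate.
; E passes through that gate to display the widget, then removes it after a short delay.
; Leaving the box disables input and closes the gate.
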(event `Key|E`
  (params (Key :type "Key Structure"))
  ;[1 1 1] Interaction (Talk)
  (:`Pressed`
    (`/Engine/EditorBlueprintResources/StandardMacros.Gate` true :!label _label
      (:`Exit`
        (`UserWidget.AddToViewport` (stale `self.Box.OnComponentBeginOverlap` _returnvalue) 0)
        (`KismetSystemLibrary.Delay` 3.0)
        (`Widget.RemoveFromParent` (stale `self.Box.OnComponentBeginOverlap` _returnvalue))))))

(event `self.Box.OnComponentBeginOverlap`
  (params (OverlappedComponent :type "PrimitiveComponent Object Reference") (OtherActor :type "Actor Object Reference") (OtherComp :type "PrimitiveComponent Object Reference") (OtherBodyIndex :type Integer) (bFromSweep :type Boolean) (SweepResult :type "HitResult Structure (by ref)"))
  ;[1 1 1] Interaction (Talk)
  (cast `/Game/Blueprints/CharacterBlueprints/BP_Player` OtherActor)
  (`self.EnableInput` (`GameplayStatics.GetPlayerController` 0))
  (bind _returnvalue (`|CreateWidget` "/Game/Blueprints/HistoryWidgets/WBP_History.WBP_History_C"))
  (set `/Game/Blueprints/HistoryWidgets/WBP_History.Interaction Text` (`self.Interaction Text`) _returnvalue)
  (goto _label :!via `Open`))

(event `self.Box.OnComponentEndOverlap`
  (params (OverlappedComponent :type "PrimitiveComponent Object Reference") (OtherActor :type "Actor Object Reference") (OtherComp :type "PrimitiveComponent Object Reference") (OtherBodyIndex :type Integer))
  ;[1 1 1] Interaction (Talk)
  (cast `/Game/Blueprints/CharacterBlueprints/BP_Player` OtherActor)
  (`self.DisableInput` (`GameplayStatics.GetPlayerController` 0))
  (goto _label :!via `Close`))

(fn `UserConstructionScript`)