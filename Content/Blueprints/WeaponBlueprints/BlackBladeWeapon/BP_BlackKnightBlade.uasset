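; BP_BlackKnightBlade is a world pickup for the Black Knight blade weapon.
; Overlap events on InteractionBox show InteractionKeyText while BP_Player is inside and hide it on exit.
; PickupWeapon removes the mesh and interaction box, then displays a history widget filled with InteractionText for two seconds before destroying the actor.
; No logic here grants or equips the weapon, and nothing in the graph calls PickupWeapon.
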(event `self.InteractionBox.OnComponentBeginOverlap`
  (params (OverlappedComponent :type "PrimitiveComponent Object Reference") (OtherActor :type "Actor Object Reference") (OtherComp :type "PrimitiveComponent Object Reference") (OtherBodyIndex :type Integer) (bFromSweep :type Boolean) (SweepResult :type "HitResult Structure (by ref)"))
  ;[1 1 1] Set Visible/Hidden Interaction Text
  (cast `/Game/Blueprints/CharacterBlueprints/BP_Player` OtherActor)
  (`SceneComponent.SetHiddenInGame` (`self.Interaction Key Text`) false false))

(event `self.InteractionBox.OnComponentEndOverlap`
  (params (OverlappedComponent :type "PrimitiveComponent Object Reference") (OtherActor :type "Actor Object Reference") (OtherComp :type "PrimitiveComponent Object Reference") (OtherBodyIndex :type Integer))
  ;[1 1 1] Set Visible/Hidden Interaction Text
  (cast `/Game/Blueprints/CharacterBlueprints/BP_Player` OtherActor)
  (`SceneComponent.SetHiddenInGame` (`self.Interaction Key Text`) true false))

(event `/Game/Blueprints/WeaponBlueprints/Interface/WeaponInterface.Pickup Weapon`
  ;[1 1 1] Player Picking Up Item
  (`ActorComponent.K2_DestroyComponent` (`self.StaticMeshComponent0`))
  (`ActorComponent.K2_DestroyComponent` (`self.InteractionBox`))
  (bind _returnvalue (`|CreateWidget` "/Game/Blueprints/HistoryWidgets/WBP_History.WBP_History_C"))
  (set `/Game/Blueprints/HistoryWidgets/WBP_History.Interaction Text` (`self.Interaction Text`) _returnvalue)
  (`UserWidget.AddToViewport` _returnvalue 0)
  (`KismetSystemLibrary.Delay` 2.0)
  (`Widget.RemoveFromParent` _returnvalue)
  (`self.K2_DestroyActor`))

(fn `UserConstructionScript`)