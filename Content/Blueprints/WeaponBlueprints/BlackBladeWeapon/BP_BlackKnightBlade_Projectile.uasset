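; Projectile for the Black Knight Blade weapon that damages enemies it hits.
; On spawn it plays a swoosh sound, then destroys itself after a fixed lifetime.
; Collision hits ignore the owner and BP_Player; any other hit zeroes the ProjectileMovement velocity and passes ATK to actors implementing EnnemyInterface.
; A hit does not destroy the projectile, which remains until its lifetime ends.
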(event `self.ReceiveBeginPlay`
  ;[1 1 1] LifeTime
  (`GameplayStatics.PlaySound2D` "/Game/Assets/SFX/clean-fast-swooshaiff-14784.clean-fast-swooshaiff-14784" 0.5 1.0 0.0 null null)
  (`KismetSystemLibrary.Delay` 7.5)
  (`self.K2_DestroyActor`))

(event `self.Collision.OnComponentHit`
  (params (HitComponent :type "PrimitiveComponent Object Reference") (OtherActor :type "Actor Object Reference") (OtherComp :type "PrimitiveComponent Object Reference") (NormalImpulse :type "Vector Structure") (Hit :type "HitResult Structure (by ref)"))
  ;[1 1 1] Velocity System When Collide
  (if (not (== OtherActor (`self.GetOwner`)))
    (cast `/Game/Blueprints/CharacterBlueprints/BP_Player` OtherActor
      (:`CastFailed`
        (set `MovementComponent.Velocity` (0.0 0.0 0.0) (`self.ProjectileMovement`))
        (if (`KismetSystemLibrary.DoesImplementInterface` OtherActor "/Game/Blueprints/NPCBlueprints/Interface/EnnemyInterface.EnnemyInterface_C")
          (bind _asennemy_interface (cast `/Game/Blueprints/NPCBlueprints/Interface/EnnemyInterface` OtherActor))
          (`/Game/Blueprints/NPCBlueprints/Interface/EnnemyInterface.Taking Damage Event Occurs` _asennemy_interface (`self.ATK`)))))))

(fn `UserConstructionScript`)